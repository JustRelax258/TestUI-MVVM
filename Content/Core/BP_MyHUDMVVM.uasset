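; BP_MyHUDMVVM sets up the main UI and its view model when play begins, likely as the game's HUD class.
; On BeginPlay it creates WBP_MainMV, adds it to the viewport and switches the player to UI-only input with a visible cursor.
; It then constructs an MV_Main and registers it in the MVVM game subsystem's global collection under context name "1", after the widget is already created.
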(event `self.ReceiveBeginPlay`
  (bind _returnvalue (`GameplayStatics.GetPlayerController` 0))
  (bind _returnvalue_2 (`|CreateWidget` "/Game/MVVM/UI/WBP_MainMV.WBP_MainMV_C"))
  (bind _output_get (set `self.WBP_MainMVVM` _returnvalue_2))
  (`UserWidget.AddToViewport` _output_get 0)
  (`WidgetBlueprintLibrary.SetInputMode_UIOnlyEx` _returnvalue null)
  (set `PlayerController.bShowMouseCursor` true _returnvalue)
  (bind _returnvalue_3 (`|GenericCreateObject` "/Game/MVVM/MV_Main.MV_Main_C"))
  (bind _returnvalue_4 (`MVVMViewModelCollectionObject.AddViewModelInstance` (`MVVMGameSubsystem.GetViewModelCollection` (subsystem `MVVMGameSubsystem`)) (make `MVVMViewModelContext` "/Game/MVVM/MV_Main.MV_Main_C" "1") _returnvalue_3))
  (if _returnvalue_4
    (`KismetSystemLibrary.PrintString` "ViewModel created in GameMode")))

(fn `UserConstructionScript`)